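; BP_Enemy is an enemy actor that keeps the BP_KillEmAllGameMode enemy count up to date.
; BeginPlay increments the count through the game mode and clears the DeathDone flag.
; Tick casts the actor itself to MyPlayer and polls IsDead, using DeathDone so the count is decremented only once on death.
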(event `self.ReceiveBeginPlay`
  (bind _asbp_kill_em_all_game_mode (cast `/Game/BP_KillEmAllGameMode` (`GameplayStatics.GetGameMode`)))
  (`/Game/BP_KillEmAllGameMode.IncreaseEnemies` _asbp_kill_em_all_game_mode)
  (set `self.DeathDone` false))

(event `self.ReceiveTick`
  (params (DeltaSeconds :type "Float (single-precision)"))
  (bind _asmy_player (cast `MyPlayer` self))
  (if (`self.IsDead` _asmy_player)
    (if (not (`self.DeathDone`))
      (set `self.DeathDone` true)
      (bind _asbp_kill_em_all_game_mode (cast `/Game/BP_KillEmAllGameMode` (`GameplayStatics.GetGameMode`)))
      (`/Game/BP_KillEmAllGameMode.DecreaseEnemies` _asbp_kill_em_all_game_mode))))

(fn `UserConstructionScript`)