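; BP_KillEmAllGameMode is a game mode that tracks the living enemy count and a growing enemy cap.
; IncreaseEnemies and DecreaseEnemies adjust EnemiesAlive by one, but nothing here spawns enemies or enforces the cap.
; Tick uses chained Delays as a repeating timer to call IncreaseLimit, which periodically multiplies MaxEnemies and truncates it, so small values may never grow.
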(event `IncreaseEnemies`
  (`/Engine/EditorBlueprintResources/StandardMacros.IncrementInt` (`self.EnemiesAlive`)))

(event `DecreaseEnemies`
  (`/Engine/EditorBlueprintResources/StandardMacros.DecrementInt` (`self.EnemiesAlive`)))

(event `IncreaseLimit`
  (params (Duration :type "Float (single-precision)") (IncrementMultiplier :type "Float (double-precision)"))
  (`KismetSystemLibrary.Delay` Duration)
  (set `self.MaxEnemies` (`KismetMathLibrary.FTrunc` (* (`self.MaxEnemies`) IncrementMultiplier))))

(event `self.ReceiveBeginPlay`)

(event `self.ReceiveTick`
  (params (DeltaSeconds :type "Float (single-precision)"))
  (`KismetSystemLibrary.Delay` 5.0)
  (`self.IncreaseLimit` 10.0 1.1))

(fn `UserConstructionScript`)