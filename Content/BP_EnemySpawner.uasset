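; Enemy spawner actor that periodically spawns BP_Enemy or BP_Enemy2 at its own location.
; BeginPlay starts a looping timer with a random interval of a few seconds, rolled once rather than per spawn.
; Each tick of the timer makes two nested coin flips, giving each enemy type a one-in-four chance and no spawn otherwise.
; Only the BP_Enemy spawn explicitly adjusts for collisions and always spawns.
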(event `self.ReceiveBeginPlay`
  (`KismetSystemLibrary.K2_SetTimerDelegate` (delegate `SpawnEnemy`) (`KismetMathLibrary.RandomFloatInRange` 5.0 8.0) true))

(event `SpawnEnemy`
  (switch `int` (`KismetMathLibrary.RandomIntegerInRange` 0 1)
    (:`0`
      (switch `int` (`KismetMathLibrary.RandomIntegerInRange` 0 1)
        (:`1`
          (`|SpawnActorFromClass` "/Game/BP_Enemy2.BP_Enemy2_C" (`KismetMathLibrary.MakeTransform` (`self.K2_GetActorLocation`)) "Undefined" "MultiplyWithRoot" null null))))
    (:`1`
      (switch `int` (`KismetMathLibrary.RandomIntegerInRange` 0 1)
        (:`1`
          (`|SpawnActorFromClass` "/Game/BP_Enemy.BP_Enemy_C" (`KismetMathLibrary.MakeTransform` (`self.K2_GetActorLocation`)) "AdjustIfPossibleButAlwaysSpawn" "MultiplyWithRoot" null null))))))

(fn `UserConstructionScript`)